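; Trigger actor for a scripted "find the child" scare sequence in which a skeletal mesh flickers between placed points as the third-person player advances.
; The first overlap turns on the player's custom depth and starts step one; later Box1 overlaps advance a counter, hiding the mesh at a far point and flickering it at the next.
; At the final step, possession flashes between First and Third pawns, then stays on First and initializes it.
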(event OnComponentBeginOverlap(Box1)
  (params (OtherActor :type Actor%20Object%20Reference) (OtherComp :type Primitive%20Component%20Object%20Reference) (OtherBodyIndex :type Integer) (bFromSweep :type Boolean) (SweepResult :type Hit%20Result%20Structure%20%28by%20ref%29))
  (bind _returnvalue (Game|GetPlayerController 0))
  (bind _first (Variables|Default|GetFirst))
  (Utilities|Casting|CastToThirdPersonCharacter OtherActor)
  (switch int (Variables|Default|GetSequencia)
    (:1
      (Transformation|SetWorldTransform (Variables|Default|GetSkeletalMesh) (Transformation|GetActorTransform (Variables|Default|GetPointLejos)) false false)
      (CallFunction|Secuencia2))
    (:2
      (Transformation|SetWorldTransform (Variables|Default|GetSkeletalMesh) (Transformation|GetActorTransform (Variables|Default|GetPointLejos)) false false)
      (CallFunction|Secuencia3))
    (:3
      (CallFunction|Flash 0.05)
      (Utilities|FlowControl|Delay 2.0)
      (CallFunction|Flash 0.1)
      (Utilities|FlowControl|Delay 0.2)
      (CallFunction|Flash 0.05)
      (Utilities|FlowControl|Delay 0.2)
      (CallFunction|Flash 0.1)
      (Utilities|FlowControl|Delay 1.0)
      (Pawn|UnPossess _returnvalue)
      (Pawn|Possess _returnvalue _first)
      (Default|Init _first))))

(event Custom|Secuencia2
  (Transformation|SetWorldTransform (Variables|Default|GetSkeletalMesh) (Transformation|GetActorTransform (Variables|Default|GetPoint2)) false false)
  (Utilities|FlowControl|Delay 0.2)
  (Transformation|SetWorldTransform (Variables|Default|GetSkeletalMesh) (Transformation|GetActorTransform (Variables|Default|GetPointLejos)) false false)
  (Utilities|FlowControl|Delay 0.2)
  (Transformation|SetWorldTransform (Variables|Default|GetSkeletalMesh) (Transformation|GetActorTransform (Variables|Default|GetPoint2)) false false)
  (Math|Integer|IncrementInt (Variables|Default|GetSequencia)))

(event Custom|Flash
  (params (Time :type Float%20%28single-precision%29))
  (bind _returnvalue (Game|GetPlayerController 0))
  (bind _returnvalue_2 (Game|GetPlayerController 0))
  (Pawn|UnPossess _returnvalue_2)
  (Pawn|Possess _returnvalue_2 (Variables|Default|GetFirst))
  (Utilities|FlowControl|Delay Time)
  (Pawn|UnPossess _returnvalue)
  (Pawn|Possess _returnvalue (Variables|Default|GetThird)))

(event Custom|Secuencia3
  (Transformation|SetWorldTransform (Variables|Default|GetSkeletalMesh) (Transformation|GetActorTransform (Variables|Default|GetPoint3)) false false)
  (Utilities|FlowControl|Delay 0.2)
  (Transformation|SetWorldTransform (Variables|Default|GetSkeletalMesh) (Transformation|GetActorTransform (Variables|Default|GetPointLejos)) false false)
  (Utilities|FlowControl|Delay 0.2)
  (Transformation|SetWorldTransform (Variables|Default|GetSkeletalMesh) (Transformation|GetActorTransform (Variables|Default|GetPoint3)) false false)
  (Math|Integer|IncrementInt (Variables|Default|GetSequencia)))

(event Custom|Secuencia1
  (Transformation|SetWorldTransform (Variables|Default|GetSkeletalMesh) (Transformation|GetActorTransform (Variables|Default|GetPoint1)) false false)
  (Utilities|FlowControl|Delay 0.2)
  (Transformation|SetWorldTransform (Variables|Default|GetSkeletalMesh) (Transformation|GetActorTransform (Variables|Default|GetPointLejos)) false false)
  (Utilities|FlowControl|Delay 0.2)
  (Transformation|SetWorldTransform (Variables|Default|GetSkeletalMesh) (Transformation|GetActorTransform (Variables|Default|GetPoint1)) false false)
  (Math|Integer|IncrementInt (Variables|Default|GetSequencia)))

(event EventBeginPlay
  (Transformation|SetWorldTransform (Variables|Default|GetSkeletalMesh) (Transformation|GetActorTransform (Variables|Default|GetPointLejos)) false false))

(event EventActorBeginOverlap
  (params (OtherActor :type Actor%20Object%20Reference))
  (Utilities|FlowControl|DoOnce false
    (:Completed
      (bind _asthird_person_character (Utilities|Casting|CastToThirdPersonCharacter OtherActor))
      (Rendering|SetRenderCustomDepth (Variables|/Script/Engine.Character|GetMesh _asthird_person_character) true)
      (CallFunction|Secuencia1)
      (Development|PrintString "Sequencia"))))

(event EventTick
  (params (DeltaSeconds :type Float%20%28single-precision%29)))

(fn ConstructionScript)