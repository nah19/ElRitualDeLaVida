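; BP_Autobot is an actor with a Box collision component and two meshes, currently acting as a collision test.
; Actor overlap, Box overlap and Box hit events all feed one debug PrintString.
; An unconnected DoOnce branch would create dynamic material instances for both meshes and raise their Emissive parameter to make them glow, but it never runs.
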(event OnComponentBeginOverlap(Box)
  (params (OtherActor :type Actor%20Object%20Reference) (OtherComp :type Primitive%20Component%20Object%20Reference) (OtherBodyIndex :type Integer) (bFromSweep :type Boolean) (SweepResult :type Hit%20Result%20Structure%20%28by%20ref%29))
  (Development|PrintString "OVERLAPPPP"))

(event OnComponentHit(Box)
  (params (OtherActor :type Actor%20Object%20Reference) (OtherComp :type Primitive%20Component%20Object%20Reference) (NormalImpulse :type Vector :default "0, 0, 0") (Hit :type Hit%20Result%20Structure%20%28by%20ref%29))
  (Development|PrintString "OVERLAPPPP"))

(event EventBeginPlay)

(event EventActorBeginOverlap
  (params (OtherActor :type Actor%20Object%20Reference))
  (Development|PrintString "OVERLAPPPP"))

(event EventTick
  (params (DeltaSeconds :type Float%20%28single-precision%29)))

(fn ConstructionScript)