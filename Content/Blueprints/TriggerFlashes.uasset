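; Trigger actor that plays a one-time sequence of brief perspective flashes when any actor first overlaps it.
; A DoOnce on begin overlap calls the Flash event four times, separated by delays, with varying short durations.
; Each flash makes player controller 0 possess the First pawn, wait briefly, then possess the Third pawn, using possession swaps as the flash effect.
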(event Custom|Flash
  (params (Time :type Float%20%28single-precision%29))
  (bind _returnvalue (Game|GetPlayerController 0))
  (bind _returnvalue_2 (Game|GetPlayerController 0))
  (Pawn|UnPossess _returnvalue_2)
  (Pawn|Possess _returnvalue_2 (Variables|Default|GetFirst))
  (Utilities|FlowControl|Delay Time)
  (Pawn|UnPossess _returnvalue)
  (Pawn|Possess _returnvalue (Variables|Default|GetThird)))

(event EventBeginPlay)

(event EventActorBeginOverlap
  (params (OtherActor :type Actor%20Object%20Reference))
  (Utilities|FlowControl|DoOnce false
    (:Completed
      (CallFunction|Flash 0.05)
      (Utilities|FlowControl|Delay 2.0)
      (CallFunction|Flash 0.1)
      (Utilities|FlowControl|Delay 0.2)
      (CallFunction|Flash 0.05)
      (Utilities|FlowControl|Delay 0.2)
      (CallFunction|Flash 0.1))))

(event EventTick
  (params (DeltaSeconds :type Float%20%28single-precision%29)))

(fn ConstructionScript)