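; BP_TriggerInicio is a one-shot overlap trigger that plays an intro cinematic with the title HUD.
; On overlap, it sends the ThirdPersonCharacter toward Point, sets its UnderWind flag, slows global time, plays a Matinee and blends to MatineeCamera.
; After timed delays it adds HUD_TITULO, then restores normal time, blends back to the character and hides the Fog.
; DoOnce precedes the cast, so any first overlapping actor consumes it.
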(event EventBeginPlay)

(event EventActorBeginOverlap
  (params (OtherActor :type Actor%20Object%20Reference))
  (Utilities|FlowControl|DoOnce false
    (:Completed
      (bind _asthird_person_character (Utilities|Casting|CastToThirdPersonCharacter OtherActor))
      (AI|Navigation|SimpleMovetoLocation (Pawn|GetController _asthird_person_character) (Transformation|GetActorLocation (Variables|Default|GetPoint)))
      (Variables|/Game/ThirdPersonBP/Blueprints/ThirdPersonCharacter.ThirdPersonCharacter_C|SetUnderWind _asthird_person_character true)
      (Utilities|Time|SetGlobalTimeDilation 0.2)
      (Audio|Components|Audio|Play (Variables|Default|GetMatinee))
      (Game|Player|SetViewTargetwithBlend (Game|GetPlayerController 0) (Variables|Default|GetMatineeCamera) 1.0 "VTBlend_Cubic" 0.0 false)
      (Utilities|FlowControl|Delay 2.0)
      (bind _returnvalue (UserInterface|CreateWidget "/Game/Widget/HUD_TITULO.HUD_TITULO_C" (Game|GetPlayerController 0)))
      (UserInterface|Viewport|AddtoViewport _returnvalue 100)
      (Utilities|FlowControl|Delay 3.0)
      (Utilities|Time|SetGlobalTimeDilation 1.0)
      (Game|Player|SetViewTargetwithBlend (Game|GetPlayerController 0) _asthird_person_character 1.0 "VTBlend_Cubic" 0.0 false)
      (Rendering|SetVisibility (Variables|/Script/Engine.ExponentialHeightFog|GetComponent (Variables|Default|GetFog)) false false))))

(event EventTick
  (params (DeltaSeconds :type Float%20%28single-precision%29)))

(fn ConstructionScript)