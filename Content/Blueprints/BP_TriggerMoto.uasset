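; BP_TriggerMoto is a trigger actor that hands player control from the third-person character to a FirstPerson pawn.
; When a ThirdPersonCharacter overlaps it, a timeline drives an extreme bloom intensity on that character's FollowCamera as a screen transition.
; When the timeline finishes, player controller 0 unpossesses, possesses the referenced FirstPerson pawn and calls its Init.
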(event EventBeginPlay)

(event EventActorBeginOverlap
  (params (OtherActor :type Actor%20Object%20Reference))
  (bind _returnvalue (Game|GetPlayerController 0))
  (bind _firstperson (Variables|Default|GetFirstPerson))
  (bind _asthird_person_character (Utilities|Casting|CastToThirdPersonCharacter OtherActor))
  (bind _newtrack_0 (Timeline|Timeline_0 Play)
    (:Update
      (Variables|/Script/Engine.CameraComponent|SetPostProcessSettings (Variables|/Game/ThirdPersonBP/Blueprints/ThirdPersonCharacter.ThirdPersonCharacter_C|GetFollowCamera _asthird_person_character) (Utilities|Struct|MakePostProcessSettings true (* _newtrack_0 1e+05))))
    (:Finished
      (Pawn|UnPossess _returnvalue)
      (Pawn|Possess _returnvalue _firstperson)
      (Default|Init _firstperson 1))))

(event EventTick
  (params (DeltaSeconds :type Float%20%28single-precision%29)))

(fn ConstructionScript)