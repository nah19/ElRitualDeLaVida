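; TriggerTrans is a one-shot trigger actor that lights up two placed meshes and plays an Optimus Prime message sound.
; The first actor overlap passes a DoOnce, prints a debug string, then creates dynamic material instances for both referenced meshes with a very high Emissive value.
; It applies them to slot 0 and plays the sound loudly at the first mesh's location, with no check on the overlapping actor.
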(event EventBeginPlay)

(event EventActorBeginOverlap
  (params (OtherActor :type Actor%20Object%20Reference))
  (bind _mesh (Variables|Default|GetMesh))
  (bind _mesh2 (Variables|Default|GetMesh2))
  (Utilities|FlowControl|DoOnce false
    (:Completed
      (Development|PrintString "OVERLAPPPP")
      (bind _returnvalue (Rendering|Material|CreateDynamicMaterialInstance (Variables|/Script/Engine.StaticMeshActor|GetStaticMeshComponent _mesh) 0 (Rendering|Material|GetMaterial (Variables|/Script/Engine.StaticMeshActor|GetStaticMeshComponent _mesh) 0) :!class /Script/Engine.PrimitiveComponent))
      (Rendering|Material|SetScalarParameterValue _returnvalue "Emissive" 5e+02 :!class /Script/Engine.MaterialInstanceDynamic)
      (bind _returnvalue_2 (Rendering|Material|CreateDynamicMaterialInstance (Variables|/Script/Engine.StaticMeshActor|GetStaticMeshComponent _mesh2) 0 (Rendering|Material|GetMaterial (Variables|/Script/Engine.StaticMeshActor|GetStaticMeshComponent _mesh2) 0) :!class /Script/Engine.PrimitiveComponent))
      (Rendering|Material|SetScalarParameterValue _returnvalue_2 "Emissive" 5e+02 :!class /Script/Engine.MaterialInstanceDynamic)
      (Rendering|Material|SetMaterial (Variables|/Script/Engine.StaticMeshActor|GetStaticMeshComponent _mesh2) 0 _returnvalue_2)
      (Rendering|Material|SetMaterial (Variables|/Script/Engine.StaticMeshActor|GetStaticMeshComponent _mesh) 0 _returnvalue)
      (Audio|PlaySoundatLocation "/Game/Audio/Optimus_prime_manda_un_mensaje.Optimus_prime_manda_un_mensaje" (Transformation|GetActorLocation (Variables|Default|GetMesh)) "0, 0, 0" 2e+01))))

(event EventTick
  (params (DeltaSeconds :type Float%20%28single-precision%29)))

(fn ConstructionScript)