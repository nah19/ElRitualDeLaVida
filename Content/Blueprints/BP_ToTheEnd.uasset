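; BP_ToTheEnd is an overlap trigger that teleports the ThirdPersonCharacter to the transform of a referenced SpawnPoint actor.
; On overlap, it disables camera boom lag, teleports without sweep, hides the Fog component and activates a particle system.
; Camera lag is restored after a short delay, so the camera snaps with the teleport.
; Movement-stop and Altar material color nodes are left unconnected and never run.
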(event EventBeginPlay)

(event EventActorBeginOverlap
  (params (OtherActor :type Actor%20Object%20Reference))
  (bind _asthird_person_character (Utilities|Casting|CastToThirdPersonCharacter OtherActor))
  (Variables|/Script/Engine.SpringArmComponent|SetbEnableCameraLag (Variables|/Game/ThirdPersonBP/Blueprints/ThirdPersonCharacter.ThirdPersonCharacter_C|GetCameraBoom _asthird_person_character) false)
  (Transformation|SetActorTransform OtherActor (Transformation|GetActorTransform (Variables|Default|GetSpawnPoint)) false true)
  (Rendering|SetVisibility (Variables|/Script/Engine.ExponentialHeightFog|GetComponent (Variables|Default|GetFog)) false false)
  (Components|Activation|Activate (Variables|/Script/Engine.Emitter|GetParticleSystemComponent (Variables|Default|GetParticles)) false)
  (Utilities|FlowControl|Delay 0.5)
  (Variables|/Script/Engine.SpringArmComponent|SetbEnableCameraLag (Variables|/Game/ThirdPersonBP/Blueprints/ThirdPersonCharacter.ThirdPersonCharacter_C|GetCameraBoom _asthird_person_character) true))

(event EventTick
  (params (DeltaSeconds :type Float%20%28single-precision%29)))

(fn ConstructionScript)