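; FinalTrigger is a trigger actor that appears meant to pick an outcome from the player's karma.
; Actor begin overlap and Box end overlap toggle an Inside flag, with no filter on the overlapping actor.
; EPressed prints debug text and, when Inside, tests the first ThirdPersonCharacter's KARMA against two thresholds for three tiers.
; All three branches are empty, so no outcome happens yet.
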(event OnComponentEndOverlap(Box)
  (params (OtherActor :type Actor%20Object%20Reference) (OtherComp :type Primitive%20Component%20Object%20Reference) (OtherBodyIndex :type Integer))
  (Variables|Default|SetInside false))

(event Custom|EPressed
  (Development|PrintString "EPRESSEd")
  (bind _outactors (Actor|GetAllActorsOfClass "/Game/ThirdPersonBP/Blueprints/ThirdPersonCharacter.ThirdPersonCharacter_C"))
  (if (Variables|Default|GetInside)
    (Development|PrintString "INSIDE")
    (if (not (< (Variables|/Game/ThirdPersonBP/Blueprints/ThirdPersonCharacter.ThirdPersonCharacter_C|GetKARMA (Utilities|Array|Get(acopy) _outactors)) 3.3))
      (if (< (Variables|/Game/ThirdPersonBP/Blueprints/ThirdPersonCharacter.ThirdPersonCharacter_C|GetKARMA (Utilities|Array|Get(acopy) _outactors)) 6.6)
        _))))

(event EventBeginPlay)

(event EventActorBeginOverlap
  (params (OtherActor :type Actor%20Object%20Reference))
  (Variables|Default|SetInside true))

(event EventTick
  (params (DeltaSeconds :type Float%20%28single-precision%29)))

(fn ConstructionScript)